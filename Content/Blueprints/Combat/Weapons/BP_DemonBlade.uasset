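; BP_DemonBlade is a melee weapon actor that deals magic damage to actors it overlaps.
; On overlap it ignores its parent actor, adds a particle effect using the hit actor's transform and applies a small fixed damage with the MagicDamage type.
; Damage is credited to the controller of the parent actor's instigator, so the blade relies on being a child actor of its wielder.
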(event `self.ReceiveActorBeginOverlap`
  (params (OtherActor :type "Actor Object Reference"))
  (bind _returnvalue (`self.GetParentActor`))
  (`parent.ReceiveActorBeginOverlap` OtherActor)
  (if (!= OtherActor _returnvalue)
    (`AddComponent|NODE_AddParticleSystemComponent-1` :`bManualAttachment` true :`RelativeTransform` (`self.GetTransform` OtherActor))
    (`GameplayStatics.ApplyDamage` OtherActor 5.0 (`Pawn.GetController` (`Actor.Instigator` _returnvalue)) self "/Game/Blueprints/Combat/Damage/MagicDamage.MagicDamage_C")))

(fn `UserConstructionScript`
  (`parent.UserConstructionScript`))