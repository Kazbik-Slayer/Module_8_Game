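; BP_NightEdge is a combat weapon Blueprint that customizes the damage calculation inherited from its parent.
; Its Calc Damage override takes the parent's result and switches on the current move, boosting Left Attack slightly while Right Attack and all other moves keep the base value.
; The event graph holds only disabled stubs and the construction script just calls the parent.
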(fn `Calc Damage`
  (params (`Other Actor` :type "Actor Object Reference"))
  (returns (Damage :type "Float (double-precision)"))
  (bind _damage (`parent.Calc Damage` `Other Actor`))
  (switch `name` (`self.Current Move`)
    (:`Default`
      _)
    (:`RigthAttack`
      _)
    (:`LeftAttack`
      (return (* _damage 1.1))))
  (return _damage))

(fn `UserConstructionScript`
  (`parent.UserConstructionScript`))