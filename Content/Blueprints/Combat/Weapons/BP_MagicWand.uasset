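; BP_MagicWand is a magic weapon Blueprint that launches a projectile when its responsive phase ends.
; EndResponsive calls the parent, computes damage, then spawns ProjectileClass at the mesh's projectile socket, aimed along the parent actor's ArrowComponent.
; The spawn passes a ProjectileInfo struct carrying damage, magic damage type, launcher and initial speed.
; BeginResponsive only defers to the parent, and the event graph holds just disabled stubs.
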(fn `Begin Responsive`
  (`parent.Begin Responsive`))

(fn `End Responsive`
  (`parent.End Responsive`)
  (bind _damage (`self.Calc Damage` null))
  (`|SpawnActorFromClass` (`self.Projectile Class`) (`KismetMathLibrary.MakeTransform` (`SceneComponent.GetSocketLocation` (`self.StaticMesh`) (`self.Projectile Socket Name`)) (`SceneComponent.K2_GetComponentRotation` (`self.GetComponentByClass` (`self.GetParentActor`) "/Script/Engine.ArrowComponent"))) "Undefined" "OverrideRootScale" null (make `/Game/Blueprints/Combat/Projectiles/ProjectileInfo` _damage "/Game/Blueprints/Combat/Damage/MagicDamage.MagicDamage_C" self 800.0) (`self.Instigator`)))

(fn `UserConstructionScript`
  (`parent.UserConstructionScript`))