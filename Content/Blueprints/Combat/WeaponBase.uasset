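; Base weapon actor that damages actors it overlaps, ignoring its parent actor.
; Damage sums the weapon's Stats damage, defaulted in the construction script, and the parent's StatsComponent damage, crediting the parent's instigator controller.
; With UseUniqueOverlap, a HaveOverlapped list limits hits to one per actor until BeginResponsive clears it.
; EndResponsive is empty, and each hit prints a debug string.
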(event `self.ReceiveTick`
  (params (DeltaSeconds :type "Float (single-precision)")))

(event `self.ReceiveActorBeginOverlap`
  (params (OtherActor :type "Actor Object Reference"))
  (bind _returnvalue (`self.GetParentActor`))
  (bind _have_overlapped (`self.Have Overlapped`))
  (if (!= OtherActor _returnvalue)
    (if (`self.Use Unique Overlap?`)
      (if (not (`BlueprintSetLibrary.Set_Contains` _have_overlapped OtherActor))
        (`BlueprintSetLibrary.Set_Add` _have_overlapped OtherActor)
        (bind _damage (`self.Calc Damage` :!label _label))
        (bind _returnvalue_2 (`GameplayStatics.ApplyDamage` OtherActor _damage (`Pawn.GetController` (`Actor.Instigator` _returnvalue)) self (`self.Damage Type`)))
        (`KismetSystemLibrary.PrintString` (`KismetStringLibrary.JoinStringArray` (`|MakeArray` (`KismetStringLibrary.Conv_DoubleToString` _returnvalue_2) (`KismetSystemLibrary.GetDisplayName` OtherActor)))))
      (else
        (goto _label)))))

(fn `Begin Responsive`
  (`BlueprintSetLibrary.Set_Clear` (`self.Have Overlapped`)))

(fn `Calc Damage`
  (returns (Damage :type "Float (double-precision)"))
  (return (+ (`.Damage_6_7214F67D426802730FB7E897D28015E4` (break `/Game/Blueprints/Combat/StatsModel` (`/Game/Blueprints/Combat/StatsComponent.Stats` (`self.GetComponentByClass` (`self.GetParentActor`) "/Game/Blueprints/Combat/StatsComponent.StatsComponent_C")))) (`.Damage_6_7214F67D426802730FB7E897D28015E4` (break `/Game/Blueprints/Combat/StatsModel` (`self.Stats`))))))

(fn `End Responsive`)

(fn `UserConstructionScript`
  ;[1 1 1] Need to be initialized using some assets
  (setmembers `/Game/Blueprints/Combat/StatsModel` :`StructRef` (`self.Stats`) :`Damage` 10.0 :`DamageDealAmp` 1.0))