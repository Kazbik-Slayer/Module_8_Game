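; Player controller Blueprint that turns the controlled pawn toward the world point under the mouse cursor on the Targeting input.
; Press and release each trigger a single rotation step; Tick is empty, so holding does not keep rotating.
; The step traces Visibility under the cursor, interpolates toward the look-at rotation and applies only yaw.
; Interp speed is the character movement's yaw rotation rate scaled by delta time.
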(event `self.ReceiveTick`
  (params (DeltaSeconds :type "Float (single-precision)")))

(event `InputAction|Targeting`
  (params (Key :type "Key Structure"))
  (:`Pressed`
    (`self.rotate To Mouse 2DLocation` (* (`GameplayStatics.GetWorldDeltaSeconds`) (.yaw (`CharacterMovementComponent.RotationRate` (`Character.CharacterMovement` (`GameplayStatics.GetPlayerCharacter` 0))))) :!label _label))
  (:`Released`
    (goto _label)))

(fn `rotate To Mouse 2DLocation`
  (params (`Interp Speed` :type "Float (double-precision)"))
  (locals (`Delta Yaw` :type "Float (double-precision)") (Direction :type "Float (double-precision)" :default 1.0))
  (bind _returnvalue (`self.K2_GetPawn`))
  (`self.K2_SetActorRotation` (`self.K2_GetPawn`) (`KismetMathLibrary.MakeRotator` 0.0 0.0 (.yaw (`KismetMathLibrary.RInterpTo` (`self.K2_GetActorRotation` _returnvalue) (`KismetMathLibrary.FindLookAtRotation` (`self.K2_GetActorLocation` _returnvalue) (`.Location` (`GameplayStatics.BreakHitResult` (`self.GetHitResultUnderCursorByChannel` "TraceTypeQuery1")))) (`GameplayStatics.GetWorldDeltaSeconds`) `Interp Speed`))) false))

(fn `UserConstructionScript`)