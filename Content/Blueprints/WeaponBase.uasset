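; Base weapon actor that damages actors it overlaps, ignoring the parent actor that wields it.
; On overlap it calls CalcDamage, which sums the parent's StatsModel and its own base damage, but ApplyDamage receives no damage amount.
; The parent's instigator controller is credited, and debug strings print each result.
; The construction script initializes the weapon's base damage; BeginResponsive and EndResponsive are empty stubs.
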(event `self.ReceiveTick`
  (params (DeltaSeconds :type "Float (single-precision)")))

(event `self.ReceiveActorBeginOverlap`
  (params (OtherActor :type "Actor Object Reference"))
  (bind _returnvalue (`self.GetParentActor`))
  (`KismetSystemLibrary.PrintString` "Weapon overlaped")
  (if (!= OtherActor _returnvalue)
    (`self.Calc Damage`)
    (bind _returnvalue_2 (`GameplayStatics.ApplyDamage` OtherActor 0.0 (`Pawn.GetController` (`Actor.Instigator` _returnvalue)) self "/Script/Engine.DamageType"))
    (`KismetSystemLibrary.PrintString` (`KismetStringLibrary.JoinStringArray` (`|MakeArray` (`KismetStringLibrary.Conv_DoubleToString` _returnvalue_2) (`KismetSystemLibrary.GetDisplayName` OtherActor))))
    (else
      (`KismetSystemLibrary.PrintString` "Self Overlap"))))

(fn `Begin Responsive`)

(fn `Calc Damage`
  (returns (Damage :type "Float (double-precision)"))
  (return (+ (`StatsModel.BaseDamage` (`self.GetComponentByClass` (`self.GetParentActor`) "/Script/Project.StatsModel")) (`StatsModel.BaseDamage` (`self.Stats`)))))

(fn `End Responsive`)

(fn `UserConstructionScript`
  (set `StatsModel.BaseDamage` 1.0 (`self.Stats`)))