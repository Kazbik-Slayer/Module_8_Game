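; Base unit character with health stats, damage handling, death and revival, and primary and secondary attacks.
; Attack inputs pass DoOnce gates to empty attack functions, while start and end events toggle weapon responsiveness and end events re-arm the gates.
; Damage is scaled by type-specific resistance, and zero health disables collision.
; Tick uses DoOnce gates to destroy the corpse after a delay, or restore collision if the unit is alive again.
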(event `InputAction|Attack`
  (params (Key :type "Key Structure"))
  (:`Pressed`
    (`/Engine/EditorBlueprintResources/StandardMacros.DoOnce` false :!label _label
      (:`Completed`
        (`self.On Attack`)))))

(event `InputAction|Secondary Attack`
  (params (Key :type "Key Structure"))
  (:`Pressed`
    (`/Engine/EditorBlueprintResources/StandardMacros.DoOnce` false :!label _label_2
      (:`Completed`
        (`self.On Secondary Attack`)))))

(event `End Attack`
  (`|ExecutionSequence`
    (:`then_0`
      (`self.Toggle Weapon Responsiveness` (`self.Weapon`) :!label _label_3))
    (:`then_1`
      (goto _label :!via `Reset`))))

(event `End Secondary Attack`
  (`|ExecutionSequence`
    (:`then_0`
      (`self.Toggle Weapon Responsiveness` (`self.Secondary Weapon`) :!label _label_4))
    (:`then_1`
      (goto _label_2 :!via `Reset`))))

(event `Start Attack`
  (goto _label_3 :!via `On Start`))

(event `Start Secondary Attack`
  (goto _label_4 :!via `On Start`))

(event `self.ReceiveAnyDamage`
  (params (Damage :type "Float (single-precision)") (DamageType :type "DamageType Object Reference") (InstigatedBy :type "Controller Object Reference") (DamageCauser :type "Actor Object Reference"))
  (bind _asmy_damage_type_base (cast `/Game/Blueprints/Combat/Utilities/MyDamageTypeBase` DamageType))
  (`self.DamageReaction` Damage _asmy_damage_type_base InstigatedBy DamageCauser))

(event `self.ReceiveTick`
  (params (DeltaSeconds :type "Float (single-precision)"))
  (if (not (`self.IsAlive?`))
    (`|ExecutionSequence`
      (:`then_0`
        (`/Engine/EditorBlueprintResources/StandardMacros.DoOnce` false :!label _label_5
          (:`Completed`
            (`KismetSystemLibrary.RetriggerableDelay` (`self.Couspe Expire Time`))
            (if (not (`self.IsAlive?`))
              (`self.K2_DestroyActor`)
              (`self.Unit Destroyed`)))))
      (:`then_1`
        (goto _label_6 :!via `Reset`)))
    (else
      (`|ExecutionSequence`
        (:`then_0`
          (`/Engine/EditorBlueprintResources/StandardMacros.DoOnce` true :!label _label_6
            (:`Completed`
              (`self.Unit Rrevival`))))
        (:`then_1`
          (goto _label_5 :!via `Reset`))))))

(event `Unit Destroyed`)

(event `Unit Rrevival`
  (`PrimitiveComponent.SetCollisionEnabled` (`self.CapsuleComponent`) "QueryAndPhysics"))

(fn `DamageReaction`
  (params (Damage :type "Float (double-precision)") (DamageType :type "/Game/Blueprints/Combat/Utilities/MyDamageTypeBase Object Reference") (InstigatedBy :type "Controller Object Reference") (DamageCauser :type "Actor Object Reference"))
  (locals (DamageAmount :type "Float (double-precision)"))
  (bind _stats_ref (`self.Stats Ref`))
  (bind (_health _mana _damage _damagedealamp _damagetakeamp _magicresist _physicalresist) (break `/Game/Blueprints/Combat/StatsModel` (`self.Stats Ref`)))
  (bind _returnvalue (* _damagetakeamp Damage))
  (if (`self.IsAlive?`)
    (switch `/Game/Blueprints/Combat/Utilities/EDamageTypes` (`/Game/Blueprints/Combat/Utilities/MyDamageTypeBase.TypeName` DamageType)
      (:`NewEnumerator0`
        (set `local.DamageAmount` (* _magicresist _returnvalue)))
      (:`NewEnumerator1`
        (set `local.DamageAmount` (* _physicalresist _returnvalue)))
      (:`NewEnumerator2`
        (set `local.DamageAmount` _returnvalue)))
    (setmembers `/Game/Blueprints/Combat/StatsModel` :`StructRef` _stats_ref :`Health` (- (`.Health_2_1C6D91BE4EB1E99B6DDEA896349BE096` (break `/Game/Blueprints/Combat/StatsModel` _stats_ref)) (`local.DamageAmount`)))
    (if (> (`.Health_2_1C6D91BE4EB1E99B6DDEA896349BE096` (break `/Game/Blueprints/Combat/StatsModel` (`self.Stats Ref`))) 0.0)
      (`KismetSystemLibrary.PrintString` (`KismetStringLibrary.Conv_DoubleToString` (`.Health_2_1C6D91BE4EB1E99B6DDEA896349BE096` (break `/Game/Blueprints/Combat/StatsModel` (`self.Stats Ref`)))) true true (struct :`R` 1.0 :`G` 0.051854 :`B` 0.07175 :`A` 1.0))
      (else
        (`self.On Death`)))))

(fn `On Attack`
  (return))

(fn `On Death`
  (set `self.IsAlive?` false)
  (`PrimitiveComponent.SetCollisionEnabled` (`self.CapsuleComponent`) "NoCollision"))

(fn `On Secondary Attack`
  (return))

(fn `UserConstructionScript`
  ;[1 1 1] need to be uploaded from some assets
  (bind _stats (`/Game/Blueprints/Combat/StatsComponent.Assign` (`self.Stats Component`) (make `/Game/Blueprints/Combat/StatsModel` 100.0 100.0 10.0 1.0 1.0 1.0 1.0)))
  (set `self.Stats Ref` _stats))