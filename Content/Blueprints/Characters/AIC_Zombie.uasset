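; AI controller for zombies that makes the pawn wander randomly around its spawn location.
; Shortly after BeginPlay it caches the controlled BP_Zombie and its location, then enables wandering.
; A DoOnce on Tick issues AI MoveTo toward a random point in a flat box around spawn.
; On success or failure it waits, prints the result, adds a fixed movement input and resets the gate for the next move.
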(event `self.ReceiveBeginPlay`
  (`KismetSystemLibrary.Delay` 0.2)
  (set `self.BPZombie` (cast `/Game/Blueprints/Characters/BP_Zombie` (`self.K2_GetPawn`) :!pure true))
  (set `self.SpawnLocation` (`self.K2_GetActorLocation` (cast `/Game/Blueprints/Characters/BP_Zombie` (`self.K2_GetPawn`) :!pure true)))
  (set `self.PauseToStart` true))

(event `self.ReceiveTick`
  (params (DeltaSeconds :type "Float (single-precision)"))
  (if (`self.PauseToStart`)
    (`/Engine/EditorBlueprintResources/StandardMacros.DoOnce` false :!label _label
      (:`Completed`
        (bind _movementresult (`|AIMoveTo` (`self.BPZombie`) (`KismetMathLibrary.RandomPointInBoundingBox` (`self.SpawnLocation`) (1600.0 1600.0 0.0)) null)
          (:`OnSuccess`
            _)
          (:`OnFail`
            _))
        (`KismetSystemLibrary.Delay` 1.0)
        (`KismetSystemLibrary.PrintString` (`|GetEnumeratorNameAsString` _movementresult))
        (`Pawn.AddMovementInput` (`self.BPZombie`) (1231.0 1213.0 123.0) 1.0 true)
        (goto _label :!via `Reset`)))))

(fn `UserConstructionScript`)