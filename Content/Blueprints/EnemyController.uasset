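; Enemy AI controller that switches a possessed BaseUnitCharacter between chasing the player to attack and wandering around its spawn point.
; While the unit lives, Tick uses CanFindPlayer, which contains distance, yaw-difference and player-alive checks, to pick the move.
; An IfNotBusy macro gates each AIMoveTo until a short delay after success or failure clears the busy flag.
; DisableMoving is stored and exposed, but movement logic here ignores it.
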(event `self.ReceiveBeginPlay`)

(event `self.ReceivePossess`
  (params (PossessedPawn :type "Pawn Object Reference"))
  (set `self.SpawnLocation` (`self.K2_GetActorLocation` PossessedPawn))
  (set `self.Unit` (cast `/Game/Blueprints/Characters/BaseUnitCharacter` PossessedPawn :!pure true)))

(event `self.ReceiveTick`
  (params (DeltaSeconds :type "Float (single-precision)"))
  (bind _returnvalue (`GameplayStatics.GetPlayerCharacter` 0))
  (if (`/Game/Blueprints/Characters/BaseUnitCharacter.IsAlive?` (`self.Unit`))
    (if (`self.CanFindPlayer`)
      (`self.IfNotBusy`)
      (`|AIMoveTo` (`self.Unit`) (0.0 0.0 0.0) _returnvalue (+ (`CapsuleComponent.GetScaledCapsuleRadius` (`Character.CapsuleComponent` _returnvalue)) (`CapsuleComponent.GetScaledCapsuleRadius` (`Character.CapsuleComponent` (`self.Unit`))) (`self.Attack Range`))
        (:`OnSuccess`
          (`/Game/Blueprints/Characters/BaseUnitCharacter.Do Attack` (`self.Unit`)))
        (:`OnFail`
          _))
      (`KismetSystemLibrary.Delay` 0.5)
      (`self.ResetActionBlocks`)
      (else
        (`self.IfNotBusy`)
        (`|AIMoveTo` (`self.Unit`) (`NavigationSystemV1.K2_GetRandomLocationInNavigableRadius` (`self.SpawnLocation`) (`self.NavRadius`) null null) null
          (:`OnSuccess`
            _)
          (:`OnFail`
            _))
        (`KismetSystemLibrary.Delay` 1.0)
        (`self.ResetActionBlocks`)))))

(event `ResetActionBlocks`
  (set `self.isBusy` false))

(event `/Game/Blueprints/ControllerFlags.Set DisableMoving`
  (params (Value :type Boolean))
  (set `self.Disable Moving` Value))

(fn `Get Disable Moving`
  (returns (Value :type Boolean))
  (return (`self.Disable Moving`)))

(fn `UserConstructionScript`)