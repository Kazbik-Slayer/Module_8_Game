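; Usable tier-3 mana potion item that restores the player character's stats when used.
; The use-item override reads the PotionMana3 row from DT_Potions and adds its Health and Mana bonuses to the character's StatsComponent, capping each at its base value.
; It then plays a potion sound and attaches a mana-potion Niagara effect to the player.
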(event `self.DoUseItem (DO OVERRIDE)`
  (bind _returnvalue (`GameplayStatics.GetPlayerCharacter` 0))
  (bind _asbp_project_character (cast `/Game/Blueprints/Characters/BP_ProjectCharacter` _returnvalue))
  (bind _returnvalue_2 (`|GetDataTableRow` "/Game/InventorySystem/Datatables/DT_Potions.DT_Potions" "PotionMana3")
    (:`then`
      (bind _stats_component (`/Game/Blueprints/Characters/BaseUnitCharacter.Stats Component` _asbp_project_character))
      (bind _stats (`/Game/Blueprints/Combat/StatsComponent.Stats` _stats_component))
      (bind (_health _mana) (break `/Game/Blueprints/Combat/StatsModel` _stats))
      (bind (_health_2 _mana_2) (break `/Game/Blueprints/Combat/StatsModel` (`.AdditionalStats_6_F0EBD95E4A9EB69172691D90A5E144ED` (break `/Game/InventorySystem/Structs/FItemPotionStruct` _returnvalue_2))))
      (bind _returnvalue_3 (+ _health _health_2))
      (bind (_health_3 _mana_3) (break `/Game/Blueprints/Combat/StatsModel` (`/Game/Blueprints/Combat/StatsComponent.BaseStats` _stats_component)))
      (if (> _returnvalue_3 _health_3)
        (setmembers `/Game/Blueprints/Combat/StatsModel` :`StructRef` _stats :`Health` _health_3)
        (else
          (setmembers `/Game/Blueprints/Combat/StatsModel` :`StructRef` _stats :`Health` _returnvalue_3)))
      (bind _returnvalue_4 (+ _mana _mana_2))
      (if (> _returnvalue_4 _mana_3)
        (setmembers `/Game/Blueprints/Combat/StatsModel` :`StructRef` _stats :`Mana` _mana_3)
        (else
          (setmembers `/Game/Blueprints/Combat/StatsModel` :`StructRef` _stats :`Mana` _returnvalue_4)))
      (`GameplayStatics.PlaySound2D` "/Game/InventorySystem/ProjectExample/Blueprints/Items/Potions/Sounds/Sound_Use_Potion_Cue.Sound_Use_Potion_Cue" 1.0 1.0 0.0 null null)
      (bind _returnvalue_5 (`AddComponent|NODE_AddNiagaraComponent-0` :`self` _returnvalue))
      (`NiagaraComponent.SetAsset` _returnvalue_5 "/Game/InventorySystem/ProjectExample/Blueprints/Items/Potions/Textures/NS_Use_Potion_Mana.NS_Use_Potion_Mana" true))))

(fn `UserConstructionScript`
  (`parent.UserConstructionScript`))