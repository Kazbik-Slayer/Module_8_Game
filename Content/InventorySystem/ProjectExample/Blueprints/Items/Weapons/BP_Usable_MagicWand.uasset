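; Usable inventory item for the magic wand, which equips the wand weapon when the player uses it.
; The use event casts player 0's character and calls UseWeaponClass with BP_MagicWand as the primary weapon, then adds one item through the player state's InventoryManagerComponent.
; Potion sound and Niagara effect nodes remain in the graph but are disconnected and never run.
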(event `self.DoUseItem (DO OVERRIDE)`
  (bind _asbp_project_character (cast `/Game/Blueprints/Characters/BP_ProjectCharacter` (`GameplayStatics.GetPlayerCharacter` 0)))
  (`/Game/Blueprints/Characters/BP_ProjectCharacter.Use Weapon Class` _asbp_project_character "/Game/Blueprints/Combat/Weapons/BP_MagicWand.BP_MagicWand_C" false)
  (`/Game/InventorySystem/Blueprints/BP_InventoryManagerComponent.AddItem` (`/Game/InventorySystem/ProjectExample/Blueprints/BP_InventoryPlayerState.InventoryManagerComponent` (cast `/Game/InventorySystem/ProjectExample/Blueprints/BP_InventoryPlayerState` (`GameplayStatics.GetPlayerState` 0) :!pure true)) "NewEnumerator23" 1))

(fn `UserConstructionScript`
  (`parent.UserConstructionScript`))